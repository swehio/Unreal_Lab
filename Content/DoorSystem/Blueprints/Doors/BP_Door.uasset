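; BP_Door is an interactable physics door that stays locked until it receives a key.
; A physics constraint locks the swing at BeginPlay, and the Execute event sets HasKey.
; Interact with a key loosens the swing limit, marks the door open and plays an unlock sound, otherwise a locked sound plays.
; It supplies an E-key icon and an "Open Door" prompt that empties once open.
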(event `self.ReceiveBeginPlay`
  (`PhysicsConstraintComponent.SetAngularSwing1Limit` (`self.PhysicsConstraint`) "ACM_Locked" 0.0))

(event `/Game/LAB/Object/BI_Execute.Execute`
  (set `self.bHasKey` true))

(event `self.Interact`
  (params (Interactor :type "Actor Object Reference"))
  (if (`self.bHasKey`)
    (`PhysicsConstraintComponent.SetAngularSwing1Limit` (`self.PhysicsConstraint`) "ACM_Limited" 90.0)
    (set `self.bIsOpen` true)
    (`GameplayStatics.PlaySoundAtLocation` "/Game/LAB/Sound/UnLock.UnLock" (`SceneComponent.K2_GetComponentLocation` (`self.Door`)) (struct) 1.0 1.0 0.0 null null null null)
    (else
      (`GameplayStatics.PlaySoundAtLocation` "/Game/LAB/Sound/Lock.Lock" (`SceneComponent.K2_GetComponentLocation` (`self.Door`)) (struct) 1.0 1.0 0.0 null null null null))))

(fn `GetInteractIcon`
  (returns (ReturnValue :type "Texture2D Object Reference"))
  (return "/Game/EasyInputPrompts/GraphicContent/MouseAndKeyboard/T_Keyboard_E.T_Keyboard_E"))

(fn `GetInteractText`
  (returns (ReturnValue :type Text))
  (if (`self.bIsOpen`)
    (return "")
    (else
      (return "Open Door"))))

(fn `UserConstructionScript`
  (`parent.UserConstructionScript`))