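; BP_Door is an interactable physics door that stays locked until its Execute event grants it a key.
; A PhysicsConstraint has its Swing1 angular motion locked on BeginPlay.
; Interacting while it is not yet Available plays a lock sound without the key.
; With the key, it frees the hinge to a limited swing, plays an unlock sound, switches the Box collision profile and marks itself Available.
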(event `self.ReceiveBeginPlay`
  (`PhysicsConstraintComponent.SetAngularSwing1Limit` (`self.PhysicsConstraint`) "ACM_Locked" 0.0))

(event `/Game/LAB/Object/BI_Execute.Execute`
  (set `self.bHasKey` true))

(event `self.Interact`
  (params (Interactor :type "Actor Object Reference"))
  (if (`|EnumInequality` (`self.InteractableState`) "Available")
    (if (`self.bHasKey`)
      (`PhysicsConstraintComponent.SetAngularSwing1Limit` (`self.PhysicsConstraint`) "ACM_Limited" 90.0)
      (set `self.bIsOpen` true)
      (`GameplayStatics.PlaySoundAtLocation` "/Game/LAB/Sound/UnLock.UnLock" (`SceneComponent.K2_GetComponentLocation` (`self.Door`)) (struct) 1.0 1.0 0.0 null null null null)
      (`PrimitiveComponent.SetCollisionProfileName` (`self.Box`) "InteractableIcon" true)
      (`self.SetInteractableState` "Available")
      (else
        (`GameplayStatics.PlaySoundAtLocation` "/Game/LAB/Sound/Lock.Lock" (`SceneComponent.K2_GetComponentLocation` (`self.Door`)) (struct) 1.0 1.0 0.0 null null null null)))))

(fn `UserConstructionScript`)