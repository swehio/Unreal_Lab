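; A locked lab door that needs a key to open and swings shut automatically when an overlap with its Box ends.
; Execute grants the key; interacting while unavailable plays a lock sound, or with the key plays an unlock sound, makes it Available and refreshes the LabPlayerController interaction UI.
; Interacting once Available runs the OpenDoor timeline to rotate the door, and the overlap end reverses it.
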(event `self.OnInteraction`
  (params (`Player Ref` :type "/Game/DoorSystem/Player/Blueprints/BP_ThirdPersonCharacter Object Reference"))
  (if (`self.bHasKey`)
    (bind (_direction _door_timer) (`Timeline|OpenDoor` :!label _label)
      (:`Update`
        (`SceneComponent.K2_SetRelativeRotation` (`self.Door`) (`KismetMathLibrary.RLerp` (struct) (struct :`Yaw` 90.0) _door_timer) false false)))))

(event `self.Box.OnComponentEndOverlap`
  (params (OverlappedComponent :type "PrimitiveComponent Object Reference") (OtherActor :type "Actor Object Reference") (OtherComp :type "PrimitiveComponent Object Reference") (OtherBodyIndex :type Integer))
  (goto _label :!via `Reverse`))

(event `/Game/LAB/Object/BI_Execute.Execute`
  (set `self.bHasKey` true))

(event `self.Interact`
  (params (Interactor :type "Actor Object Reference"))
  (if (`|EnumInequality` (`self.InteractableState`) "Available")
    (if (`self.bHasKey`)
      (set `self.bIsOpen` true)
      (`GameplayStatics.PlaySoundAtLocation` "/Game/LAB/Sound/UnLock.UnLock" (`SceneComponent.K2_GetComponentLocation` (`self.Door`)) (struct) 1.0 1.0 0.0 null null null null)
      (`self.SetInteractableState` "Available")
      (bind _aslab_player_controller (cast `LabPlayerController` (`GameplayStatics.GetPlayerController` 0)))
      (`LabPlayerController.UpdateInteractionUI` _aslab_player_controller)
      (else
        (`GameplayStatics.PlaySoundAtLocation` "/Game/LAB/Sound/Lock.Lock" (`SceneComponent.K2_GetComponentLocation` (`self.Door`)) (struct) 1.0 1.0 0.0 null null null null)))
    (else
      (`/Game/DoorSystem/Player/Blueprints/BI_Interact.OnInteraction` null))))

(fn `UserConstructionScript`)