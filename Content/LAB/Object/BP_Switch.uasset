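; BP_Switch is an interactable switch that flips between two positions and signals a linked Light.
; Interact calls ToggleSwitch, where a FlipFlop alternates the Switch component's relative transform between default and tilted rotation.
; It then calls ExecuteMessage on Light and plays the switch sound at the Switch's world location.
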(event `self.ReceiveBeginPlay`)

(event `ToggleSwitch`
  (bind _switch (`self.Switch`))
  (`/Engine/EditorBlueprintResources/StandardMacros.FlipFlop`
    (:`A`
      (`SceneComponent.K2_SetRelativeTransform` _switch (`KismetMathLibrary.MakeTransform` (0.0 0.0 0.0)) false false))
    (:`B`
      (`SceneComponent.K2_SetRelativeTransform` _switch (`KismetMathLibrary.MakeTransform` (0.0 0.0 0.0) (struct :`Pitch` 20.0)) false false))))

(event `self.Interact`
  (params (Interactor :type "Actor Object Reference"))
  (`self.ToggleSwitch`)
  (message `/Game/LAB/Object/BI_Execute.Execute` (`self.Light`))
  (`GameplayStatics.PlaySoundAtLocation` "/Game/LAB/Sound/SC_Switch.SC_Switch" (`SceneComponent.K2_GetComponentLocation` (`self.Switch`)) (struct) 1.0 1.0 0.0 null null null null))

(fn `UserConstructionScript`)